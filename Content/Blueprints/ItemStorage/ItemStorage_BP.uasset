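; Item storage Blueprint that holds an inventory of items and a gold, silver and copper purse.
; On BeginPlay it fills the storage array with InventorySlot widgets, which hold the slot data themselves.
; AddItem stacks stackable items onto matching slots with room, otherwise using the first empty slot; a separate function moves whole stacks.
; AddGold merges a gold bag's coins, carries overflow past 99 upward, then destroys the bag actor.
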(event EventBeginPlay
  (CallFunction|InitStorage))

(fn ConstructionScript)

(fn AddItem
  (params (Item :type Base%20Item%20BP%20Object%20Reference))
  (bind _output_get (LocalVariables|SetTempItem Item))
  ;[1 1 1] Is the new item stackable? If not, there is no point in searching for existing items in the storage so just add it to the inventory
  (if (Variables|/Game/Blueprints/ItemStorage/BaseItem_BP.BaseItem_BP_C|GetStackable _output_get)
    (for _array_element (Variables|Default|GetStorage)
      ;[1 1 1] Loop through the whole storage and try to find any occurance of the same item with space in the stack, if you find one, add this item to the stack and finish execution of the function
      (if (not (Variables|/Game/Blueprints/ItemStorage/InventorySlot.InventorySlot_C|GetSlotEmpty _array_element))
        (if (and (Utilities|Name|Equal(Name) (Variables|/Game/Blueprints/ItemStorage/BaseItem_BP.BaseItem_BP_C|GetItemID (Variables|/Game/Blueprints/ItemStorage/InventorySlot.InventorySlot_C|GetItem _array_element)) (Variables|/Game/Blueprints/ItemStorage/BaseItem_BP.BaseItem_BP_C|GetItemID (LocalVariables|GetTempItem))) (< (Variables|/Game/Blueprints/ItemStorage/InventorySlot.InventorySlot_C|GetStackSize _array_element) (Variables|Default|GetMaxStackSize)))
          (bind _successful (Default|AddItemtoStack _array_element (LocalVariables|GetTempItem)))
          (if _successful
            (return true)))))
    ;[1 1 1] We have looped through the whole storage and haven't found items so will add a new one to the storage
    (bind _successful_2 (CallFunction|StroreNewItem (LocalVariables|GetTempItem)))
    (return _successful_2)
    (else
      (bind _successful_3 (CallFunction|StroreNewItem (LocalVariables|GetTempItem)))
      (return _successful_3))))

(fn StroreNewItem
  (params (Item :type Base%20Item%20BP%20Object%20Reference))
  (LocalVariables|SetTempItem Item)
  ;[1 1 1] Loop through the storage and find the first empty slot and add the item to that slot. If there is no emptry slot, return error message.
  (for _array_element (Variables|Default|GetStorage)
    (if (Variables|/Game/Blueprints/ItemStorage/InventorySlot.InventorySlot_C|GetSlotEmpty _array_element)
      (Default|StoreItem _array_element (LocalVariables|GetTempItem))
      (return true)))
  ;[1 1 1] Return false as the adding operation was not successful and write the error message to the screen
  (Development|PrintString "Inventory is Full!" true true "(R=1.000000,G=0.000000,B=0.000000,A=1.000000)")
  (return false))

(fn MoveItemtoFirstEmptySlot
  (params (Item :type Base%20Item%20BP%20Object%20Reference) (StockSize :type Integer))
  (LocalVariables|SetTempStackSize StockSize)
  (LocalVariables|SetTempItem Item)
  ;[1 1 1] Loop through the storage and find the first empty slot and add the item to that slot. If there is no emptry slot, return error message.
  (for _array_element (Variables|Default|GetStorage)
    (if (Variables|/Game/Blueprints/ItemStorage/InventorySlot.InventorySlot_C|GetSlotEmpty _array_element)
      (Default|MoveItemtoSlot _array_element (LocalVariables|GetTempItem) (LocalVariables|GetTempStackSize))
      (return true)))
  ;[1 1 1] Return false as the adding operation was not successful and write the error message to the screen
  (Development|PrintString "Inventory is Full!" true true "(R=1.000000,G=0.000000,B=0.000000,A=1.000000)")
  (return false))

(fn InitStorage
  ;[1 1 1] Initiate the storage with empty slots
  (for _index (range 0 (- (Variables|Default|GetInventorySize) 1))
    (bind _returnvalue (UserInterface|CreateWidget "/Game/Blueprints/ItemStorage/InventorySlot.InventorySlot_C" 0 0 (Variables|Default|GetMaxStackSize)))
    (Utilities|Array|Add (Variables|Default|GetStorage) _returnvalue)))

(fn AddGold
  (params (Goldbag :type Goldbag%20Actor%20Object%20Reference))
  (Utilities|IsValid Goldbag ; check if we hace received a goldbag actor
    (:Is%20Valid
      ;[1 1 1 0.3] Add existing values and new values together and store the im temp variable for later use
      (LocalVariables|SetTempGold (+ (Variables|/Game/Actors/Items/GoldBag/Goldbag_Actor.Goldbag_Actor_C|GetGold Goldbag) (.Gold (Utilities|Struct|BreakGold_S (Variables|Default|GetGold)))))
      (LocalVariables|SetTempSilver (+ (Variables|/Game/Actors/Items/GoldBag/Goldbag_Actor.Goldbag_Actor_C|GetSilver Goldbag) (.Silver (Utilities|Struct|BreakGold_S (Variables|Default|GetGold)))))
      (LocalVariables|SetTempCopper (+ (Variables|/Game/Actors/Items/GoldBag/Goldbag_Actor.Goldbag_Actor_C|GetCopper Goldbag) (.Copper (Utilities|Struct|BreakGold_S (Variables|Default|GetGold)))))
      ;[1 1 1 0.3] Check if we have a surplus on copper or silver, if yes, increment the next higher value by one and finally store everything the the gold structure
      (if (> (LocalVariables|GetTempCopper) 99)
        (Math|Integer|IncrementInt (LocalVariables|GetTempSilver)
          (:%20%20
            (LocalVariables|SetTempCopper (- (LocalVariables|GetTempCopper) 100)))))
      (if (> (LocalVariables|GetTempSilver) 99)
        (Math|Integer|IncrementInt (LocalVariables|GetTempGold)
          (:%20%20
            (LocalVariables|SetTempSilver (- (LocalVariables|GetTempSilver) 100)))))
      (Variables|Default|SetGold (Utilities|Struct|MakeGold_S (LocalVariables|GetTempGold) (Math|Integer|Min(Integer) (LocalVariables|GetTempSilver) 99) (Math|Integer|Min(Integer) (LocalVariables|GetTempCopper) 99)))
      (Actor|DestroyActor Goldbag) ; Finally destroy the goldbag actor as we only need values from it
    )))