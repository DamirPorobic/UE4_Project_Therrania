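; QuestManager_BP holds the player's quest log, capped at MaxQuests, with functions to add, query, progress, turn in and abandon quests.
; AddQeust rejects duplicates, and AddToCounter advances running quests matching a target ID, marking them finished at the required quantity.
; TurnInQuest checks any quest-giver requirement, then grants item, gold and experience to Hero_BP.
; Adding, turn-in and abandoning also update the QuestTracker stored in TopDownGameInstance.
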(event EventBeginPlay)

(event EventActorBeginOverlap
  (params (OtherActor :type Actor%20Object%20Reference)))

(event EventTick
  (params (DeltaSeconds :type Float%20%28single-precision%29)))

(fn ConstructionScript)

(fn AddQeust
  (params (Quest :type Quest%20S%20Structure))
  (if (< (Utilities|Array|Length (Variables|Default|GetQuests)) (Variables|Default|GetMaxQuests)) ; Check if we have enough space for another quest
    (for _array_element (Variables|Default|GetQuests)
      ;[1 1 1 0.3] Checking for duplicate quest
      (if (Utilities|Name|Equal(Name) (Utilities|Struct|BreakQuest_S _array_element) (Utilities|Struct|BreakQuest_S Quest)) ; Compare current new QuestID with quests in log, if metch, return false and stop execution
        (return false)))
    (bind _structout (Utilities|Struct|SetmembersinQuest_S Quest "NewEnumerator1")) ; Set the state to running as we have collected the quest
    (Utilities|Array|Add (Variables|Default|GetQuests) _structout) ; Add the quest to the array
    ;[1 1 1 0.3] Add quest to the tracker
    (bind _astop_down_game_instance (Utilities|Casting|CastToTopDownGameInstance (Game|GetGameInstance)) ; Get reference to game instance as we store there all trackers
      (:then
        (bind _successful (Default|AddQuestRunning (Variables|/Game/Blueprints/TopDownGameInstance.TopDownGameInstance_C|GetQuestTracker _astop_down_game_instance) (Utilities|Struct|BreakQuest_S _structout))) ; Add the quest as running to the tracker
        (return _successful))
      (:CastFailed
        (return false)))
    (else
      (Development|PrintString "Your quest log is full, you can't take anymore quests" true true "(R=1.000000,G=0.000000,B=0.000000,A=1.000000)") ; We have no space for more quests, return false
      (return false))))

(fn HasQuest
  (params (QuestID :type Name))
  (for _array_element (Variables|Default|GetQuests)
    (if (Utilities|Name|Equal(Name) (.QuestID (Utilities|Struct|BreakQuest_S _array_element)) QuestID) ; Check if there is any quest with the provided ID, if yes, return true
      (return true)))
  (return false) ; We have looped through the whole array and haven't found any quest with that ID, so there is no such quest and we return false.
)

(fn AddtoCounter
  (params (ActorID :type Name))
  (for (_array_element _array_index) (Variables|Default|GetQuests) ; Loop through array, but don't stop at much but loop through all quests
    (if (and (Utilities|Enum|Equal(Enum) (.QuestState (Utilities|Struct|BreakQuest_S _array_element)) "NewEnumerator1") (Utilities|Name|Equal(Name) (.TargetID (Utilities|Struct|BreakQuest_S _array_element)) ActorID)) ; Check if the quest is running and if the target ID is matching
      (bind _output_get (LocalVariables|SetTempQuest _array_element))
      (bind _structout (Utilities|Struct|SetmembersinQuest_S _output_get (+ (.QuantityDone (Utilities|Struct|BreakQuest_S _array_element)) 1))) ; Increment the quantity of the quest counter
      (Utilities|Array|SetArrayElem (Variables|Default|GetQuests) _array_index _structout true) ; Put it back into the array
      (if (== (.QuantityRequired (Utilities|Struct|BreakQuest_S (LocalVariables|GetTempQuest))) (.QuantityDone (Utilities|Struct|BreakQuest_S (LocalVariables|GetTempQuest)))) ; Check if we have the required quantity, if yes, the quest is finished
        (bind _structout_2 (Utilities|Struct|SetmembersinQuest_S (LocalVariables|GetTempQuest) "NewEnumerator2")) ; Set quest to finished
        (Utilities|Array|SetArrayElem (Variables|Default|GetQuests) _array_index _structout_2 true) ; Store it back into the array
      ))))

(fn TurninQuest
  (params (QuestID :type Name) (AtQuestGiver :type Name))
  ;[1 1 1 0.3] Loop through array and search for quest
  (for _array_element (Variables|Default|GetQuests) ; Loop through array, search for the quest
    (if (and (Utilities|Enum|Equal(Enum) (.QuestState (Utilities|Struct|BreakQuest_S _array_element)) "NewEnumerator2") (Utilities|Name|Equal(Name) (.QuestID (Utilities|Struct|BreakQuest_S _array_element)) QuestID)) ; Check if the quest we want to turn in is finished
      ;[1 1 1 0.3] Check if quest needs to be return to quest giver, if yes, if the one we are talking to is the quest giver
      (if (not (.ReturnQuest (Utilities|Struct|BreakQuest_S _array_element)))
        _
        (elif (Utilities|Name|Equal(Name) (.QuestGiver (Utilities|Struct|BreakQuest_S _array_element)) AtQuestGiver)
          _
          (else
            (Development|PrintString "This quest needs to be return to thew quest giver") ; If he's not the quest giver, return false and stop execution
            (return false))))
      ;[1 1 1 0.3] Adding rewards to hero inventory and exp acount
      (bind _ashero_bp (Utilities|Casting|CastToHero_BP (Game|Player|GetPlayerPawn 0)))
      (bind _returnvalue (Game|SpawnActorfromClass (Utilities|Struct|BreakQuest_S _array_element) (|Transform) "AdjustIfPossibleButAlwaysSpawn" 0 0)) ; Get the item class out of the quest and try to spawn reward item
      (Utilities|IsValid _returnvalue ; Check if there is any reward item
        (:Is%20Valid
          (bind _successful (Default|AddItem (Variables|/Game/Pawns/Hero/Hero_BP.Hero_BP_C|GetItemStorage _ashero_bp) _returnvalue)) ; If there is a reward item, we try to add it to inventory
          (if _successful ; If adding the item was successful, continue, otherwise stop execution
            _
            (else
              (return false))))
        (:Is%20Not%20Valid
          _))
      (Default|AddGold (Variables|/Game/Pawns/Hero/Hero_BP.Hero_BP_C|GetItemStorage _ashero_bp)) ; Add gold to her gold amount
      (Default|CalculateExperience _ashero_bp (.RewardExperience (Utilities|Struct|BreakQuest_S _array_element))) ; Add experience to hero exp amount
      ;[1 1 1 0.3] Setting quest tracker
      (bind _astop_down_game_instance (Utilities|Casting|CastToTopDownGameInstance (Game|GetGameInstance)))
      (bind _successful_2 (Default|SetQuestTurnedin (Variables|/Game/Blueprints/TopDownGameInstance.TopDownGameInstance_C|GetQuestTracker _astop_down_game_instance) (Utilities|Struct|BreakQuest_S _array_element)))
      (if _successful_2
        (bind _returnvalue_2 (Utilities|Array|RemoveItem (Variables|Default|GetQuests) _array_element)) ; Remove the quest from the log
        (return _returnvalue_2) ; Only place we return true
        (else
          (return false)))))
  (return false))

(fn AbandonQuest
  (params (QuestID :type Name))
  (for (_array_element _array_index) (Variables|Default|GetQuests) ; Loop through all quests
    (if (Utilities|Name|Equal(Name) (Utilities|Struct|BreakQuest_S _array_element) QuestID) ; Check if the QuestID is matching
      (Utilities|Array|RemoveIndex (Variables|Default|GetQuests) _array_index) ; Remove the quest from the quest list
      ;[1 1 1 0.3] Remove quest from tracker
      (bind _astop_down_game_instance (Utilities|Casting|CastToTopDownGameInstance (Game|GetGameInstance)))
      (bind _successful (Default|RemoveQuestRunning (Variables|/Game/Blueprints/TopDownGameInstance.TopDownGameInstance_C|GetQuestTracker _astop_down_game_instance) QuestID))
      (return _successful)))
  (return false))