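; QuestTracker_BP records the state of the player's quests in a Quests array of ID and state structs.
; Functions add a quest as running, look up its state (defaulting to new), mark a running quest turned in, or remove a running one.
; Each searches the array linearly by QuestID, and the mutators return a success bool, printing a message on duplicates, missing entries or invalid state changes.
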(fn ConstructionScript)

(fn AddQuestRunning
  (params (QuestID :type Name))
  (for _array_element (Variables|Default|GetQuests) ; Loop through all array element,
    (if (Utilities|Name|Equal(Name) (Utilities|Struct|BreakQuestTrackerEntry_S _array_element) QuestID) ; Check if there is already such a quest in the array
      (Development|PrintString "Quest already in tracker, returning false" false)
      (return false) ; We have found this quest, this should not happen, return false
    ))
  (Utilities|Array|Add (Variables|Default|GetQuests) (Utilities|Struct|MakeQuestTrackerEntry_S QuestID "NewEnumerator1"))
  (return true))

(fn GetQuestState
  (params (QuestID :type Name))
  (for _array_element (Variables|Default|GetQuests) ; Loop through all quest items
    (if (Utilities|Name|Equal(Name) (.QuestID (Utilities|Struct|BreakQuestTrackerEntry_S _array_element)) QuestID) ; Compare searched ID and id from array item
      (return (.QuestState (Utilities|Struct|BreakQuestTrackerEntry_S _array_element))) ; Found the quest, return its state
    ))
  (return "NewEnumerator0") ; If the quest was not found in the array, return state "new"
)

(fn SetQuestTurnedin
  (params (QuestID :type Name))
  (for (_array_element _array_index) (Variables|Default|GetQuests)
    (if (Utilities|Name|Equal(Name) (.QuestID (Utilities|Struct|BreakQuestTrackerEntry_S _array_element)) QuestID) ; find the qúest with the same ID
      (if (Utilities|Enum|Equal(Enum) (.QuestState (Utilities|Struct|BreakQuestTrackerEntry_S _array_element)) "NewEnumerator1")
        (bind _output_get (LocalVariables|SetTempStruct _array_element)) ; Assign the structure to a temp variable
        (bind _structout (Utilities|Struct|SetmembersinQuestTrackerEntry_S _output_get "NewEnumerator3")) ; Set the quest to status turned in
        (Utilities|Array|SetArrayElem (Variables|Default|GetQuests) _array_index _structout) ; Store it back into the array, same index
        (return true)
        (else
          (Development|PrintString "Quest in the array but has a different state then running, this should not happen." false) ; When we are trying to set a quest to turnedIn but it has a status other then Running, something is not good
          (return false)))))
  (Development|PrintString "We have not found the quest in the array which is being tried to finish, this should not happen." false) ; Looped through whole array but haven't found a quest with same ID
  (return false))

(fn RemoveQuestRunning
  (params (QuestID :type Name))
  (for (_array_element _array_index) (Variables|Default|GetQuests) ; Loop through all quests
    (if (Utilities|Name|Equal(Name) (.QuestID (Utilities|Struct|BreakQuestTrackerEntry_S _array_element)) QuestID) ; Check if we have a quest with the same ID
      (if (Utilities|Enum|Equal(Enum) (.QuestState (Utilities|Struct|BreakQuestTrackerEntry_S _array_element)) "NewEnumerator1") ; Only rwmovw thw quest if the state is running
        (Utilities|Array|RemoveIndex (Variables|Default|GetQuests) _array_index) ; Remove quest from array
        (return true) ; Return true for successful operation
        (else
          (Development|PrintString "Trying to remove a quest which is in some other state then running is not allowed." false)
          (return false)))))
  (Development|PrintString "Trying to remove a quest which is not in the array is not allowed." false)
  (return false))