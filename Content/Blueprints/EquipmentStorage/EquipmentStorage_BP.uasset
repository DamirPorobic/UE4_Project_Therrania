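; Equipment storage that holds the player's equipment slots and totals the stats of equipped items.
; On BeginPlay it creates nine typed EquipmentSlot widgets with hardcoded character-window padding, only the first having a socket (Weapon1h).
; UpdateAttributes rebuilds the attribute totals from filled slots, copies bonus health and mana to Hero_BP's separate Additional variables, then starts health restoration.
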(event `self.ReceiveBeginPlay`
  (`self.InitStorage`))

(fn `InitStorage`
  (`|ExecutionSequence`
    (:`then_0`
      ;[1 1 1] Create a new equipment slot widget for every equipment piece that we can equip, set the type and padding so that we can position it correctly in the character window and in the end add it to the Equipment Array
      (bind _returnvalue (`|CreateWidget` "/Game/Blueprints/EquipmentStorage/EquipmentSlot.EquipmentSlot_C" null "NewEnumerator0" "Weapon1h" (make `Margin` 40.0 330.0) self))
      (`KismetArrayLibrary.Array_Add` (`self.Equipment`) _returnvalue))
    (:`then_1`
      (bind _returnvalue_2 (`|CreateWidget` "/Game/Blueprints/EquipmentStorage/EquipmentSlot.EquipmentSlot_C" null "NewEnumerator8" "None" (make `Margin` 167.0 25.0) self))
      (`KismetArrayLibrary.Array_Add` (`self.Equipment`) _returnvalue_2))
    (:`then_2`
      (bind _returnvalue_3 (`|CreateWidget` "/Game/Blueprints/EquipmentStorage/EquipmentSlot.EquipmentSlot_C" null "NewEnumerator1" "None" (make `Margin` 167.0 220.0) self))
      (`KismetArrayLibrary.Array_Add` (`self.Equipment`) _returnvalue_3))
    (:`then_3`
      (bind _returnvalue_4 (`|CreateWidget` "/Game/Blueprints/EquipmentStorage/EquipmentSlot.EquipmentSlot_C" null "NewEnumerator2" "None" (make `Margin` 330.0 240.0) self))
      (`KismetArrayLibrary.Array_Add` (`self.Equipment`) _returnvalue_4))
    (:`then_4`
      (bind _returnvalue_5 (`|CreateWidget` "/Game/Blueprints/EquipmentStorage/EquipmentSlot.EquipmentSlot_C" null "NewEnumerator3" "None" (make `Margin` 60.0 150.0) self))
      (`KismetArrayLibrary.Array_Add` (`self.Equipment`) _returnvalue_5))
    (:`then_5`
      (bind _returnvalue_6 (`|CreateWidget` "/Game/Blueprints/EquipmentStorage/EquipmentSlot.EquipmentSlot_C" null "NewEnumerator4" "None" (make `Margin` 167.0 340.0) self))
      (`KismetArrayLibrary.Array_Add` (`self.Equipment`) _returnvalue_6))
    (:`then_6`
      (bind _returnvalue_7 (`|CreateWidget` "/Game/Blueprints/EquipmentStorage/EquipmentSlot.EquipmentSlot_C" null "NewEnumerator5" "None" (make `Margin` 100.0 550.0) self))
      (`KismetArrayLibrary.Array_Add` (`self.Equipment`) _returnvalue_7))
    (:`then_7`
      (bind _returnvalue_8 (`|CreateWidget` "/Game/Blueprints/EquipmentStorage/EquipmentSlot.EquipmentSlot_C" null "NewEnumerator6" "None" (make `Margin` 167.0 120.0) self))
      (`KismetArrayLibrary.Array_Add` (`self.Equipment`) _returnvalue_8))
    (:`then_8`
      (bind _returnvalue_9 (`|CreateWidget` "/Game/Blueprints/EquipmentStorage/EquipmentSlot.EquipmentSlot_C" null "NewEnumerator7" "None" (make `Margin` 300.0 330.0) self))
      (`KismetArrayLibrary.Array_Add` (`self.Equipment`) _returnvalue_9))))

(fn `UpdateAttributes`
  (bind (_strength _armor _agility _focus _intellect _spirit _stamina _health _mana) (break `/Game/Pawns/Attributes_Struct` (`self.Attributes`)))
  (bind (_strength_2 _armor_2 _agility_2 _focus_2 _intellect_2 _spirit_2 _stamina_2 _health_2 _mana_2) (break `/Game/Pawns/Attributes_Struct` (`self.Attributes`)))
  ;[1 1 1] Zero out current stats so that we have a clean start
  (set `self.Attributes` (make `/Game/Pawns/Attributes_Struct` 0.0))
  ;[1 1 1] Loop through all equipment slots, check if they're empty, if not, add their stats to all stats
  (for _array_element (`self.Equipment`)
    (if (not (`/Game/Blueprints/EquipmentStorage/EquipmentSlot.IsSlotEmpty` _array_element))
      (bind (_strength_3 _armor_3 _agility_3 _focus_3 _intellect_3 _spirit_3 _stamina_3 _health_3 _mana_3) (break `/Game/Pawns/Attributes_Struct` (`/Game/Blueprints/ItemStorage/BaseEquipmentItem_BP.Stats` (`/Game/Blueprints/EquipmentStorage/EquipmentSlot.Equipment` _array_element))))
      (set `self.Attributes` (make `/Game/Pawns/Attributes_Struct` (+ _strength_3 _strength) (+ _armor_3 _armor) (+ _agility_3 _agility) (+ _focus_3 _focus) (+ _intellect_3 _intellect) (+ _spirit_3 _spirit) (+ _stamina_3 _stamina) (+ _health_3 _health) (+ _mana_3 _mana)))))
  (bind _ashero_bp (cast `/Game/Pawns/Hero/Hero_BP` (`GameplayStatics.GetPlayerCharacter` 0)))
  (set `/Game/Pawns/BaseCharacter.AdditionalHealth` _health_2 _ashero_bp) ; Set additional mana. It's in a seperate variable for the mana restore function to work
  (set `/Game/Pawns/BaseCharacter.AdditionalMana` _mana_2 _ashero_bp) ; Set additional health. It's in a seperate variable for the health restore function to work
  (`/Game/Pawns/BaseCharacter.StartRestoreHealth` _ashero_bp) ; Call the restore function to heal the character in case that the health has been increased by the new equipment
)

(fn `UserConstructionScript`)