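; Inventory Blueprint that stores picked items in a fixed number of slots, with stacking for stackable items.
; On BeginPlay it fills the Storage array with empty InventorySlot widgets, which hold each slot's item and stack state.
; AddItem first tops up a same-named, non-full stack, otherwise StroreNewItem fills the first empty slot.
; When no slot is free, it prints a red full-inventory message and returns false.
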(event EventBeginPlay
  ;[1 1 1] Initiate the storage with empty slots
  (for _index (range 0 (- (Variables|Default|GetInventorySize) 1))
    (bind _returnvalue (UserInterface|CreateWidget "/Game/Widgets/InventorySlot.InventorySlot_C" 0 0 (Variables|Default|GetMaxStackSize)))
    (Utilities|Array|Add (Variables|Default|GetStorage) _returnvalue)))

(fn ConstructionScript)

(fn AddItem
  (params (Item :type Base%20Item%20BP%20Object%20Reference))
  (bind _output_get (LocalVariables|SetTempItem Item))
  ;[1 1 1] Is the new item stackable? If not, there is no point in searching for existing items in the storage so just add it to the inventory
  (if (Variables|/Game/Blueprints/Inventory/BaseItem_BP.BaseItem_BP_C|GetStackable _output_get)
    (for _array_element (Variables|Default|GetStorage)
      ;[1 1 1] Loop through the whole storage and try to find any occurance of the same item with space in the stack, if you find one, add this item to the stack and finish execution of the function
      (if (not (Variables|/Game/Widgets/InventorySlot.InventorySlot_C|GetSlotEmpty _array_element))
        (if (and (Utilities|Name|Equal(Name) (Variables|/Game/Blueprints/Inventory/BaseItem_BP.BaseItem_BP_C|GetName (Variables|/Game/Widgets/InventorySlot.InventorySlot_C|GetItem _array_element)) (Variables|/Game/Blueprints/Inventory/BaseItem_BP.BaseItem_BP_C|GetName (LocalVariables|GetTempItem))) (< (Variables|/Game/Widgets/InventorySlot.InventorySlot_C|GetStackSize _array_element) (Variables|Default|GetMaxStackSize)))
          (bind _successful (Default|AddItemtoStack _array_element (LocalVariables|GetTempItem)))
          (if _successful
            (return true)))))
    ;[1 1 1] We have looped through the whole storage and haven't found items so will add a new one to the storage
    (bind _successful_2 (CallFunction|StroreNewItem (LocalVariables|GetTempItem)))
    (return _successful_2)
    (else
      (bind _successful_3 (CallFunction|StroreNewItem (LocalVariables|GetTempItem)))
      (return _successful_3))))

(fn StroreNewItem
  (params (Item :type Base%20Item%20BP%20Object%20Reference))
  (LocalVariables|SetTempItem Item)
  ;[1 1 1] Loop through the storage and find the first empty slot and add the item to that slot. If there is no emptry slot, return error message.
  (for _array_element (Variables|Default|GetStorage)
    (if (Variables|/Game/Widgets/InventorySlot.InventorySlot_C|GetSlotEmpty _array_element)
      (Default|StoreItem _array_element (LocalVariables|GetTempItem))
      (return true)))
  ;[1 1 1] Return false as the adding operation was not successful and write the error message to the screen
  (Development|PrintString "Inventory is Full!" true true "(R=1.000000,G=0.000000,B=0.000000,A=1.000000)")
  (return false))