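; ItemDropper spawns loot at its owning pawn's location, such as gold and items dropped by a killed enemy.
; Drop optionally spawns a Goldbag_Actor carrying the set gold, silver and copper, then rolls a percent chance independently for each Items entry.
; Each spawn gets a small random X/Y offset and always spawns, adjusting for collision if possible.
; Without a valid PawnOwner, it only prints a warning.
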(fn `Drop`
  (bind _returnvalue (`KismetMathLibrary.Conv_IntToDouble` (`KismetMathLibrary.RandomIntegerInRange` -8 8)))
  (bind _returnvalue_2 (`KismetMathLibrary.MakeVector` (+ (.x (`self.K2_GetActorLocation` (`self.PawnOwner`))) _returnvalue) (+ (.y (`self.K2_GetActorLocation` (`self.PawnOwner`))) _returnvalue) (.z (`self.K2_GetActorLocation` (`self.PawnOwner`)))))
  (`/Engine/EditorBlueprintResources/StandardMacros.IsValid` (`self.PawnOwner`) ; Make sure we have an owner as we need to drop the items at his location
    (:`Is Valid`
      (`|ExecutionSequence`
        (:`then_0`
          ;[1 1 1 0.3] Dropping gold
          (if (`self.DropGold`)
            (`|SpawnActorFromClass` "/Game/Actors/Items/GoldBag/Goldbag_Actor.Goldbag_Actor_C" (`KismetMathLibrary.MakeTransform` _returnvalue_2) "AdjustIfPossibleButAlwaysSpawn" "OverrideRootScale" null (`self.Gold`) (`self.Silver`) (`self.Copper`)) ; Spawn a new goldbag with gold, silver and copper amount set.
          ))
        (:`then_1`
          ;[1 1 1 0.3] Dropping items
          (for _array_element (`self.Items`)
            (bind (_item _dropchance) (break `/Game/Blueprints/ItemDropper/DropItem_S` _array_element))
            ;;[0.3 1 1 0.3] Generate a random number between 1 and 100. When the number is below the dropchance, we will spawn the item. The logic is that fo example, at the drop chance of 50% half the numbers have to be smaller then 50 whihc is a drop chance of 50%
            (if (<= (`KismetMathLibrary.RandomIntegerInRange` 1 100) _dropchance)
              (`|SpawnActorFromClass` _item (`KismetMathLibrary.MakeTransform` _returnvalue_2) "AdjustIfPossibleButAlwaysSpawn" "OverrideRootScale"))))))
    (:`Is Not Valid`
      (`KismetSystemLibrary.PrintString` "Item dropper has no owner, can't drop without location." true true (struct :`R` 1.0 :`A` 1.0) 5.0))))

(fn `UserConstructionScript`)