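; Equipment storage that holds the player's gear slots, attaches gear to the character and totals its stat bonuses.
; On BeginPlay it creates nine typed EquipmentSlot widgets with hand-placed padding for the character window; only the first names a socket.
; EquipItem unhides an item and snaps it to a Character_BP mesh socket, while UnequipItem hides and detaches it.
; Both then call UpdateStats, which re-sums occupied slots and refreshes the HUD character window.
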(event EventBeginPlay
  (CallFunction|InitStorage))

(fn ConstructionScript)

(fn InitStorage
  (Utilities|FlowControl|Sequence
    (:then_0
      ;[1 1 1] Create a new equipment slot widget for every equipment piece that we can equip, set the type and padding so that we can position it correctly in the character window and in the end add it to the Equipment Array
      (bind _returnvalue (UserInterface|CreateWidget "/Game/Widgets/EquipmentSlot.EquipmentSlot_C" 0 "NewEnumerator0" "Weapon1h" (Utilities|Struct|MakeMargin 4e+01 3.3e+02 0.0 0.0) self))
      (Utilities|Array|Add (Variables|Default|GetEquipment) _returnvalue))
    (:then_1
      (bind _returnvalue_2 (UserInterface|CreateWidget "/Game/Widgets/EquipmentSlot.EquipmentSlot_C" 0 "NewEnumerator8" "None" (Utilities|Struct|MakeMargin 167.0 25.0 0.0 0.0) self))
      (Utilities|Array|Add (Variables|Default|GetEquipment) _returnvalue_2))
    (:then_2
      (bind _returnvalue_3 (UserInterface|CreateWidget "/Game/Widgets/EquipmentSlot.EquipmentSlot_C" 0 "NewEnumerator1" "None" (Utilities|Struct|MakeMargin 167.0 2.2e+02 0.0 0.0) self))
      (Utilities|Array|Add (Variables|Default|GetEquipment) _returnvalue_3))
    (:then_3
      (bind _returnvalue_4 (UserInterface|CreateWidget "/Game/Widgets/EquipmentSlot.EquipmentSlot_C" 0 "NewEnumerator2" "None" (Utilities|Struct|MakeMargin 3.3e+02 2.4e+02 0.0 0.0) self))
      (Utilities|Array|Add (Variables|Default|GetEquipment) _returnvalue_4))
    (:then_4
      (bind _returnvalue_5 (UserInterface|CreateWidget "/Game/Widgets/EquipmentSlot.EquipmentSlot_C" 0 "NewEnumerator3" "None" (Utilities|Struct|MakeMargin 6e+01 1.5e+02 0.0 0.0) self))
      (Utilities|Array|Add (Variables|Default|GetEquipment) _returnvalue_5))
    (:then_5
      (bind _returnvalue_6 (UserInterface|CreateWidget "/Game/Widgets/EquipmentSlot.EquipmentSlot_C" 0 "NewEnumerator4" "None" (Utilities|Struct|MakeMargin 167.0 3.4e+02 0.0 0.0) self))
      (Utilities|Array|Add (Variables|Default|GetEquipment) _returnvalue_6))
    (:then_6
      (bind _returnvalue_7 (UserInterface|CreateWidget "/Game/Widgets/EquipmentSlot.EquipmentSlot_C" 0 "NewEnumerator5" "None" (Utilities|Struct|MakeMargin 1e+02 5.5e+02 0.0 0.0) self))
      (Utilities|Array|Add (Variables|Default|GetEquipment) _returnvalue_7))
    (:then_7
      (bind _returnvalue_8 (UserInterface|CreateWidget "/Game/Widgets/EquipmentSlot.EquipmentSlot_C" 0 "NewEnumerator6" "None" (Utilities|Struct|MakeMargin 167.0 1.2e+02 0.0 0.0) self))
      (Utilities|Array|Add (Variables|Default|GetEquipment) _returnvalue_8))
    (:then_8
      (bind _returnvalue_9 (UserInterface|CreateWidget "/Game/Widgets/EquipmentSlot.EquipmentSlot_C" 0 "NewEnumerator7" "None" (Utilities|Struct|MakeMargin 3e+02 3.3e+02 0.0 0.0) self))
      (Utilities|Array|Add (Variables|Default|GetEquipment) _returnvalue_9))))

(fn UpdateStats
  ;[1 1 1] Zero out current stats so that we have a clean start
  (Variables|Default|SetEquipementStats (Utilities|Struct|MakeStats_Struct 0.0 0.0))
  ;[1 1 1] Loop through all equipment slots, check if they're empty, if not, add their stats to all stats
  (for _array_element (Variables|Default|GetEquipment)
    (if (not (Variables|/Game/Widgets/EquipmentSlot.EquipmentSlot_C|GetIsSlotEmpty _array_element))
      (Variables|Default|SetEquipementStats (Utilities|Struct|MakeStats_Struct (+ (.Strength (Utilities|Struct|BreakStats_Struct (Variables|/Game/Blueprints/Inventory/BaseEquipmentItem_BP.BaseEquipmentItem_BP_C|GetStats (Variables|/Game/Widgets/EquipmentSlot.EquipmentSlot_C|GetEquipment _array_element)))) (.Strength (Utilities|Struct|BreakStats_Struct (Variables|Default|GetEquipementStats)))) (+ (.Armor (Utilities|Struct|BreakStats_Struct (Variables|/Game/Blueprints/Inventory/BaseEquipmentItem_BP.BaseEquipmentItem_BP_C|GetStats (Variables|/Game/Widgets/EquipmentSlot.EquipmentSlot_C|GetEquipment _array_element)))) (.Armor (Utilities|Struct|BreakStats_Struct (Variables|Default|GetEquipementStats)))) (+ (.Agility (Utilities|Struct|BreakStats_Struct (Variables|/Game/Blueprints/Inventory/BaseEquipmentItem_BP.BaseEquipmentItem_BP_C|GetStats (Variables|/Game/Widgets/EquipmentSlot.EquipmentSlot_C|GetEquipment _array_element)))) (.Agility (Utilities|Struct|BreakStats_Struct (Variables|Default|GetEquipementStats)))) (+ (.Focus (Utilities|Struct|BreakStats_Struct (Variables|/Game/Blueprints/Inventory/BaseEquipmentItem_BP.BaseEquipmentItem_BP_C|GetStats (Variables|/Game/Widgets/EquipmentSlot.EquipmentSlot_C|GetEquipment _array_element)))) (.Focus (Utilities|Struct|BreakStats_Struct (Variables|Default|GetEquipementStats)))) (+ (.Intellect (Utilities|Struct|BreakStats_Struct (Variables|/Game/Blueprints/Inventory/BaseEquipmentItem_BP.BaseEquipmentItem_BP_C|GetStats (Variables|/Game/Widgets/EquipmentSlot.EquipmentSlot_C|GetEquipment _array_element)))) (.Intellect (Utilities|Struct|BreakStats_Struct (Variables|Default|GetEquipementStats)))) (+ (.Spirit (Utilities|Struct|BreakStats_Struct (Variables|/Game/Blueprints/Inventory/BaseEquipmentItem_BP.BaseEquipmentItem_BP_C|GetStats (Variables|/Game/Widgets/EquipmentSlot.EquipmentSlot_C|GetEquipment _array_element)))) (.Spirit (Utilities|Struct|BreakStats_Struct (Variables|Default|GetEquipementStats)))) (+ (.Stamina (Utilities|Struct|BreakStats_Struct (Variables|/Game/Blueprints/Inventory/BaseEquipmentItem_BP.BaseEquipmentItem_BP_C|GetStats (Variables|/Game/Widgets/EquipmentSlot.EquipmentSlot_C|GetEquipment _array_element)))) (.Stamina (Utilities|Struct|BreakStats_Struct (Variables|Default|GetEquipementStats)))) (+ (.Health (Utilities|Struct|BreakStats_Struct (Variables|/Game/Blueprints/Inventory/BaseEquipmentItem_BP.BaseEquipmentItem_BP_C|GetStats (Variables|/Game/Widgets/EquipmentSlot.EquipmentSlot_C|GetEquipment _array_element)))) (.Health (Utilities|Struct|BreakStats_Struct (Variables|Default|GetEquipementStats)))) (+ (.Mana (Utilities|Struct|BreakStats_Struct (Variables|/Game/Blueprints/Inventory/BaseEquipmentItem_BP.BaseEquipmentItem_BP_C|GetStats (Variables|/Game/Widgets/EquipmentSlot.EquipmentSlot_C|GetEquipment _array_element)))) (.Mana (Utilities|Struct|BreakStats_Struct (Variables|Default|GetEquipementStats))))))))
  ;[1 1 1] Update character stats on the character window, when we change an equipment piece probably the stats have changed too
  (Default|LoadStats (Variables|/Game/Blueprints/TopDownHUD.TopDownHUD_C|GetCharacterWindow (Variables|Default|GetHUD))))

(fn EquipItem
  (params (Equipment :type Base%20Equipment%20Item%20BP%20Object%20Reference) (Socket :type Name))
  ;[1 1 1] First check if the provided item is not null and if the socket name provided really exsists, if yes, make the item visible again as it was hidden when picked up and moved to inventory. Next attach it to the socket, update equipment stats and return true for successful operation.
  (bind _output_get (LocalVariables|SetTempEquipment Equipment))
  (Utilities|IsValid _output_get
    (:Is%20Valid
      (bind _ascharacter_bp (Utilities|Casting|CastToCharacter_BP (Game|Player|GetPlayerPawn 0))
        (:then
          (if (Transformation|DoesSocketExist (Variables|/Script/Engine.Character|GetMesh _ascharacter_bp) Socket)
            (Rendering|SetActorHiddenInGame (LocalVariables|GetTempEquipment) false)
            (Class|SceneComponent|Attachto (Variables|/Game/Blueprints/Inventory/BaseItem_BP.BaseItem_BP_C|GetDefaultSceneRoot (LocalVariables|GetTempEquipment)) (Variables|/Script/Engine.Character|GetMesh _ascharacter_bp) Socket "SnapToTargetIncludingScale" false)
            (CallFunction|UpdateStats)
            (return true)
            (else
              (return false))))
        (:CastFailed
          (return false))))
    (:Is%20Not%20Valid
      (return false))))

(fn UnequipItem
  (params (Equipment :type Base%20Equipment%20Item%20BP%20Object%20Reference))
  (bind _output_get (LocalVariables|SetTempEquipment Equipment))
  (Utilities|IsValid _output_get
    (:Is%20Valid
      (Utilities|Casting|CastToCharacter_BP (Game|Player|GetPlayerPawn 0)
        (:then
          (Rendering|SetActorHiddenInGame (LocalVariables|GetTempEquipment) true)
          (Class|SceneComponent|DetachfromParent (Variables|/Game/Blueprints/Inventory/BaseItem_BP.BaseItem_BP_C|GetDefaultSceneRoot (LocalVariables|GetTempEquipment)) false true)
          (CallFunction|UpdateStats)
          (return true))
        (:CastFailed
          (return false))))
    (:Is%20Not%20Valid
      (return false))))