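; Player controller for a top-down click-to-move hero, translating mouse and key input into movement, combat, looting and UI actions.
; While GoTo is held, a gated Tick trace moves the hero to the clicked point or character; a second trace shows a hand cursor over pickups in range.
; Action loots in-range items or gold, otherwise attacks and snaps facing toward the cursor.
; Other inputs drive HUD windows, action bar slots, pause and clamped spring-arm zoom.
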(event `self.ReceiveBeginPlay`
  ;[1 1 1 0.3] Get reference to HUD and assign it to a variable for later reference
  (bind _astop_down_hud (cast `/Game/Blueprints/TopDownHUD` (`self.GetHUD`)))
  (set `self.HUD` _astop_down_hud)
  ;[1 1 1 0.3] Get reference to hero character and assign it to a variable
  (bind _ashero_bp (cast `/Game/Pawns/Hero/Hero_BP` (`GameplayStatics.GetPlayerCharacter` 0)))
  (set `self.Hero` _ashero_bp))

(event `self.ReceiveTick`
  (params (DeltaSeconds :type "Float (single-precision)"))
  (bind (_bblockinghit _binitialoverlap _time _location _impactpoint _normal _impactnormal _physmat _hitactor) (`GameplayStatics.BreakHitResult` (`self.GetHitResultUnderCursorByChannel` "TraceTypeQuery2" false)))
  (bind _ashero_bp (cast `/Game/Pawns/Hero/Hero_BP` (`GameplayStatics.GetPlayerCharacter` 0)))
  (if (not (`/Game/Pawns/BaseCharacter.IsDead` _ashero_bp))
    (`|ExecutionSequence`
      (:`then_0`
        ;[1 1 1 0.3] Movement on mouse click
        (`/Engine/EditorBlueprintResources/StandardMacros.Gate` true :!label _label ; While key is pressed...
          (:`Exit`
            (bind _asbase_character (cast `/Game/Pawns/BaseCharacter` _hitactor) ; Check if we have clicked another character (friendly or enemy)
              (:`then`
                (`self.MoveToActor` _asbase_character))
              (:`CastFailed`
                (`NavigationSystem.SimpleMoveToLocation` self _location) ; Move to clicked location
              )))))
      (:`then_1`
        ;[1 1 1 0.3] Changing cursor when hovering overn an item
        (bind _inrange (`self.ItemInRange` (`self.GetHitResultUnderCursorByChannel` "TraceTypeQuery1" false))) ; Check if it's an item and if it's in range
        (if _inrange
          (set `self.CurrentMouseCursor` "Hand")
          (else
            (set `self.CurrentMouseCursor` "Default")))))))

(event `InputAction|GoTo`
  (params (Key :type "Key Structure" :default "AnyKey"))
  ;[1 1 1 0.3] Movement on mouse click
  (:`Pressed`
    (goto _label :!via `Open`))
  (:`Released`
    (goto _label :!via `Close`)))

(event `InputAction|Action`
  (params (Key :type "Key Structure" :default "AnyKey"))
  (bind _hitresult (`self.GetHitResultUnderCursorByChannel` "TraceTypeQuery2" true))
  (bind (_bblockinghit _binitialoverlap _time _location _impactpoint _normal _impactnormal _physmat _hitactor) (`GameplayStatics.BreakHitResult` _hitresult))
  (bind _itemstorage (`/Game/Pawns/Hero/Hero_BP.ItemStorage` (`self.Hero`)))
  (:`Pressed`
    ;[1 1 1 0.3] Action handling
    (bind _ashero_bp (cast `/Game/Pawns/Hero/Hero_BP` (`GameplayStatics.GetPlayerCharacter` 0)))
    (if (not (`/Game/Pawns/BaseCharacter.IsDead` _ashero_bp))
      (bind _inrange (`self.ItemInRange` _hitresult)) ; Check if there is some item below the mouse coursor, if yes, check if it's in range
      (if _inrange
        (bind _asbase_item_bp (cast `/Game/Blueprints/ItemStorage/BaseItem_BP` _hitactor) ; Try to cast the hit object to baseItem, if possible, add the item to inventory
          (:`then`
            (`/Game/Blueprints/ItemStorage/ItemStorage_BP.AddItem` _itemstorage _asbase_item_bp) ; add item to inventory
          )
          (:`CastFailed`
            (bind _asgoldbag_actor (cast `/Game/Actors/Items/GoldBag/Goldbag_Actor` _hitactor)) ; if it's not an item then it has to be a goldbag
            (`/Game/Blueprints/ItemStorage/ItemStorage_BP.AddGoldbag` _itemstorage _asgoldbag_actor) ; Add the gold to inventory
          ))
        (else
          ;[1 1 1 0.3] Default Attack
          (bind _ashero_bp_2 (cast `/Game/Pawns/Hero/Hero_BP` (`GameplayStatics.GetPlayerCharacter` 0)))
          (`/Game/Pawns/Hero/Hero_BP.StartAttack` _ashero_bp_2) ; Call this function to trigger the base attack
          (`self.LookAtMouse` _location) ; Look at the location we have clicked
        )))))

(event `InputAction|Character Sheet`
  (params (Key :type "Key Structure" :default "AnyKey"))
  (bind _hud (`self.HUD`))
  (:`Pressed`
    ;[1 1 1 0.3] Handling open and close of character sheet
    (bind _is_character_window_open (`/Game/Blueprints/TopDownHUD.GetCharacterWindowState` (`self.HUD`)))
    (if _is_character_window_open
      (`/Game/Blueprints/TopDownHUD.CloseCharacterSheet` _hud)
      (else
        (`/Game/Blueprints/TopDownHUD.OpenCharacterSheet` _hud)))))

(event `InputAction|Inventory`
  (params (Key :type "Key Structure" :default "AnyKey"))
  (bind _hud (`self.HUD`))
  (:`Pressed`
    ;[1 1 1 0.3] Handle open and close inventory window
    (bind _isinventoryopen (`/Game/Blueprints/TopDownHUD.GetInventoryState` (`self.HUD`)))
    (if _isinventoryopen
      (`/Game/Blueprints/TopDownHUD.CloseInventory` _hud)
      (else
        (`/Game/Blueprints/TopDownHUD.OpenInventory` _hud)))))

(event `InputAction|Pause Game` :paused true
  (params (Key :type "Key Structure" :default "AnyKey"))
  (:`Pressed`
    ;[1 1 1 0.3] Pause Game
    (if (`GameplayStatics.IsGamePaused`)
      (`/Game/Blueprints/TopDownHUD.UnpauseGame` (`self.HUD`))
      (`GameplayStatics.SetGamePaused` false)
      (else
        (`/Game/Blueprints/TopDownHUD.PauseGame` (`self.HUD`))
        (`GameplayStatics.SetGamePaused` true)))))

(event `InputAction|Quest Log`
  (params (Key :type "Key Structure" :default "AnyKey"))
  (bind _hud (`self.HUD`))
  (:`Pressed`
    ;[1 1 1 0.3] Open/Close quest log window
    (bind _isquestlogopen (`/Game/Blueprints/TopDownHUD.GetQuestLogState` (`self.HUD`)))
    (if _isquestlogopen
      (`/Game/Blueprints/TopDownHUD.CloseQuestLog` _hud)
      (else
        (`/Game/Blueprints/TopDownHUD.OpenQuestLog` _hud)))))

(event `InputAction|ZoomIn`
  (params (Key :type "Key Structure" :default "AnyKey"))
  (:`Pressed`
    ;[1 1 1 0.3] Zoom in/out function
    (`self.Zoom` -100.0)))

(event `InputAction|ZoomOut`
  (params (Key :type "Key Structure" :default "AnyKey"))
  (:`Pressed`
    ;[1 1 1 0.3] Zoom in/out function
    (`self.Zoom` 100.0)))

(event `Key|One`
  (params (Key :type "Key Structure" :default "AnyKey"))
  (bind _hud (`self.HUD`))
  (:`Pressed`
    ;[1 1 1 0.3] Action bar keybinding handling
    (`/Game/Blueprints/TopDownHUD.ActionBar1_Pressed` _hud))
  (:`Released`
    (`/Game/Blueprints/TopDownHUD.ActionBar1_Released` _hud)))

(event `Key|Two`
  (params (Key :type "Key Structure" :default "AnyKey"))
  (bind _hud (`self.HUD`))
  (:`Pressed`
    ;[1 1 1 0.3] Action bar keybinding handling
    (`/Game/Blueprints/TopDownHUD.ActionBar2_Pressed` _hud))
  (:`Released`
    (`/Game/Blueprints/TopDownHUD.ActionBar2_Released` _hud)))

(event `Key|Three`
  (params (Key :type "Key Structure" :default "AnyKey"))
  (bind _hud (`self.HUD`))
  (:`Pressed`
    ;[1 1 1 0.3] Action bar keybinding handling
    (`/Game/Blueprints/TopDownHUD.ActionBar3_Pressed` _hud))
  (:`Released`
    (`/Game/Blueprints/TopDownHUD.ActionBar3_Released` _hud)))

(event `Key|Four`
  (params (Key :type "Key Structure" :default "AnyKey"))
  (bind _hud (`self.HUD`))
  (:`Pressed`
    ;[1 1 1 0.3] Action bar keybinding handling
    (`/Game/Blueprints/TopDownHUD.ActionBar4_Pressed` _hud))
  (:`Released`
    (`/Game/Blueprints/TopDownHUD.ActionBar4_Released` _hud)))

(event `Key|Five`
  (params (Key :type "Key Structure" :default "AnyKey"))
  (bind _hud (`self.HUD`))
  (:`Pressed`
    ;[1 1 1 0.3] Action bar keybinding handling
    (`/Game/Blueprints/TopDownHUD.ActionBar5_Pressed` _hud))
  (:`Released`
    (`/Game/Blueprints/TopDownHUD.ActionBar5_Released` _hud)))

(fn `ItemInRange`
  (params (Hit :type "HitResult Structure"))
  (returns (InRange :type Boolean))
  (bind (_bblockinghit _binitialoverlap _time _location _impactpoint _normal _impactnormal _physmat _hitactor) (`GameplayStatics.BreakHitResult` Hit))
  ;[1 1 1] Check if the item that we have hit is an item that can be picked up, if yes, return true if the item is in pickup range, otherwise false
  (`/Engine/EditorBlueprintResources/StandardMacros.IsValid` _hitactor ; Check if we are hitting anything
    (:`Is Valid`
      (if (`self.ActorHasTag` _hitactor "Pickup")
        (return (< (`KismetMathLibrary.VSize` (- (`self.GetFocalLocation`) _location)) (`self.ItemPickupDistance`)))
        (else
          _)))
    (:`Is Not Valid`
      _))
  (return false))

(fn `LookAtMouse`
  (params (LookAt :type "Vector Structure"))
  (bind _returnvalue (`GameplayStatics.GetPlayerPawn` 0))
  (`self.SetActorRotation` _returnvalue (`KismetMathLibrary.MakeRotator` 0.0 0.0 (+ (.yaw (`KismetMathLibrary.FindLookAtRotation` (`self.K2_GetActorLocation` _returnvalue) LookAt)) -2.0))))

(fn `MoveToActor`
  (params (Pawn :type "/Game/Pawns/BaseCharacter Object Reference"))
  ;[1 1 1 0.3] Check if we have reached the other pawn
  (if (>= (`KismetMathLibrary.VSize` (- (`self.K2_GetActorLocation` Pawn) (`self.K2_GetActorLocation` (`GameplayStatics.GetPlayerPawn` 0)))) 100.0)
    (`NavigationSystem.SimpleMoveToActor` self Pawn) ; Move to pawn if we haven't reached it yet
    (else
      (`self.LookAtMouse` (`self.K2_GetActorLocation` Pawn)) ; When we have already reached the other pawn, rotate the hero in that direction as the hero rotation is based on movement
    )))

(fn `UserConstructionScript`)

(fn `Zoom`
  (params (Delta :type "Float (double-precision)"))
  (bind _returnvalue (+ Delta (`SpringArmComponent.TargetArmLength` (`/Game/Pawns/Hero/Hero_BP.SpringArm` (`self.Hero`)))))
  (if (and (<= _returnvalue 1600.0) (>= _returnvalue 400.0))
    (set `SpringArmComponent.TargetArmLength` _returnvalue (`/Game/Pawns/Hero/Hero_BP.SpringArm` (`self.Hero`))) ; Set new value as the new spring arm lenght
  ))