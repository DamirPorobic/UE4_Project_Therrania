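; Player hero character Blueprint that handles inventory, weapon equipping, melee combat, damage reaction and leveling.
; BeginPlay spawns separate item and equipment storage actors, while attach and detach functions socket or hide gear, with only weapons implemented.
; StartAttack plays a montage when armed, and the AnimBP-timed Trigger event applies random damage to enemies overlapping the melee hitbox.
; Experience gains show floating text and trigger level-ups that randomly raise attributes and the next threshold.
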(event `self.ReceiveBeginPlay`
  ;[1 1 1 0.3] Spawn inventory actor and assign it to a variable
  (bind _returnvalue (`|SpawnActorFromClass` "/Game/Blueprints/ItemStorage/ItemStorage_BP.ItemStorage_BP_C" (`self.GetTransform`) "Undefined" "OverrideRootScale" null 36 20))
  (set `self.ItemStorage` _returnvalue)
  ;[1 1 1 0.3] Spawn equipment storage and assign it to a variable
  (bind _returnvalue_2 (`|SpawnActorFromClass` "/Game/Blueprints/EquipmentStorage/EquipmentStorage_BP.EquipmentStorage_BP_C" (`self.GetTransform`) "Undefined" "OverrideRootScale")) ; Spawn equipment storage and assign it to a variable
  (set `self.EquipmentStorage` _returnvalue_2))

(event `/Game/Pawns/iDamageable.AffectHealth`
  (params (Delta :type "Float (single-precision)") (DamageCauser :type "/Game/Pawns/BaseCharacter Object Reference"))
  ;[1 1 1 0.3] Handling damage and death
  (`self.CalculateHealth` Delta) ; Calculate damage, start restore and check if the character is dead
  (if (not (`self.IsDead`))
    (set `self.IsBeingHit` true)
    (`KismetSystemLibrary.Delay` 1.0)
    (set `self.IsBeingHit` false)))

(event `Trigger`
  ;[1 1 1 0.3] Apply damage to target
  (for _array_element (`PrimitiveComponent.GetOverlappingActors` (`self.MeleeHitBox`) "/Game/Pawns/Enemy/BaseEnemy.BaseEnemy_C")
    (bind _asbase_enemy (cast `/Game/Pawns/Enemy/BaseEnemy` _array_element)) ; Cast it to baseEnemy class which is the parent class of all enemies
    (`/Game/Pawns/Enemy/BaseEnemy.AffectHealth` _asbase_enemy (* (`KismetMathLibrary.Conv_IntToDouble` (`KismetMathLibrary.Round` (`KismetMathLibrary.RandomFloatInRange` 8.0 13.0))) -1.0) self) ; Apply damage
  ))

(fn `AttachEquipment`
  (params (Equipment :type "/Game/Blueprints/ItemStorage/BaseEquipmentItem_BP Object Reference"))
  (returns (Successful :type Boolean))
  (`/Engine/EditorBlueprintResources/StandardMacros.IsValid` Equipment ; Check if the sent item is valid
    (:`Is Valid`
      (switch `/Game/Blueprints/ItemStorage/EquipmentType_E` (`/Game/Blueprints/ItemStorage/BaseEquipmentItem_BP.EquipmentType` Equipment) ; Depending on the equipment type, do e specifc task, like setting the weapon variable to null
        (:`NewEnumerator0`
          (bind _asbase_equipment_weapon_bp (cast `/Game/Blueprints/ItemStorage/BaseEquipmentWeapon_BP` Equipment) ; Try to cast to weapon
            (:`then`
              (bind _output_get (set `self.Weapon` _asbase_equipment_weapon_bp)) ; Set it to a variable
              (`self.SetActorHiddenInGame` _output_get false) ; Set actor to visble as it has been now attached to character and should be visible
              (`SceneComponent.K2_AttachTo` (`/Game/Blueprints/ItemStorage/BaseItem_BP.DefaultSceneRoot` (`self.Weapon`)) (`self.Mesh`) (`self.Socket1hWeapon`) "SnapToTargetIncludingScale" false) ; Attach the item to the weapon socket
              (return true))
            (:`CastFailed`
              (return false))))
        (:`NewEnumerator8`
          _)
        (:`NewEnumerator1`
          _)
        (:`NewEnumerator2`
          _)
        (:`NewEnumerator3`
          _)
        (:`NewEnumerator4`
          _)
        (:`NewEnumerator5`
          _)
        (:`NewEnumerator6`
          _)
        (:`NewEnumerator7`
          _))
      (return false))
    (:`Is Not Valid`
      (return false))))

(fn `CalculateExperience`
  (params (AddExp :type "Float (double-precision)"))
  (if (> AddExp 0.0)
    ;[1 1 1 0.3] Disply amount of exp the pawn received
    (bind _asfloating_text (cast `/Game/Widgets/FloatingText` (`WidgetComponent.GetUserWidgetObject` (`self.FloatingText`))))
    (`/Game/Widgets/FloatingText.ShowText` _asfloating_text "NewEnumerator2" AddExp) ; We specify the experience text type to make the text look different then damage text
    (bind _output_get (set `self.Experience` (+ AddExp (`self.Experience`))))
    (if (>= _output_get (`self.NextLevelExperience`))
      (set `self.Experience` (- (`self.Experience`) (`self.NextLevelExperience`))) ; Check what the surplus is and set current exp to this surplus value
      (`self.LevelUp`) ; Call the level up function as we just have gained a level
    )))

(fn `DetachEquipment`
  (params (Equipment :type "/Game/Blueprints/ItemStorage/BaseEquipmentItem_BP Object Reference"))
  (`self.DetachRootComponentFromParent` Equipment false) ; Remove the equipment from the character mesh
  (switch `/Game/Blueprints/ItemStorage/EquipmentType_E` (`/Game/Blueprints/ItemStorage/BaseEquipmentItem_BP.EquipmentType` Equipment) ; Depending on what item type that was which is now removed we have to perform some special function
    (:`NewEnumerator0`
      (`self.SetActorHiddenInGame` Equipment true) ; Make the actor hidden again as it has been moved to the inventory
      (set `self.Weapon` null) ; Set the weapon variable to null as the weapon was removed
    )))

(fn `LevelUp`
  (bind (_strength _armor _agility _focus _intellect _spirit _stamina _health _mana) (break `/Game/Pawns/Attributes_Struct` (`self.Attributes`)))
  ;[1 1 1 0.3] Set new level
  (set `self.Level` (+ (`self.Level`) 1)) ; Rise level by one
  ;[1 1 1 0.3] Set new required XP for next level
  (set `self.NextLevelExperience` (`KismetMathLibrary.Conv_IntToDouble` (`KismetMathLibrary.Round` (* (`self.NextLevelExperience`) (`KismetMathLibrary.RandomFloatInRange` 3.0 5.0))))) ; We need a new NextLevelExp value, for that, we will multiply the old value by a random number from 3 to 5
  (set `self.Attributes` (make `/Game/Pawns/Attributes_Struct` (+ _strength (`KismetMathLibrary.Conv_IntToDouble` (`KismetMathLibrary.RandomInteger` 10))) (+ _armor (`KismetMathLibrary.Conv_IntToDouble` (`KismetMathLibrary.RandomInteger` 10))) (+ _agility (`KismetMathLibrary.Conv_IntToDouble` (`KismetMathLibrary.RandomInteger` 10))) (+ _focus (`KismetMathLibrary.Conv_IntToDouble` (`KismetMathLibrary.RandomInteger` 10))) (+ _intellect (`KismetMathLibrary.Conv_IntToDouble` (`KismetMathLibrary.RandomInteger` 10))) (+ _spirit (`KismetMathLibrary.Conv_IntToDouble` (`KismetMathLibrary.RandomInteger` 10))) (+ _stamina (`KismetMathLibrary.Conv_IntToDouble` (`KismetMathLibrary.RandomInteger` 10))) (+ _health (`KismetMathLibrary.Conv_IntToDouble` (`KismetMathLibrary.RandomIntegerInRange` 10 25))) (+ _mana (`KismetMathLibrary.Conv_IntToDouble` (`KismetMathLibrary.RandomIntegerInRange` 10 15))))) ; Take old attributes, add random values to them and save them as new attributes
)

(fn `StartAttack`
  (`/Engine/EditorBlueprintResources/StandardMacros.IsValid` (`self.Weapon`)
    (:`Is Valid`
      (bind _returnvalue (`self.GetCurrentMontage`))
      (`/Engine/EditorBlueprintResources/StandardMacros.IsValid` _returnvalue
        (:`Is Not Valid`
          (bind _output_get (set `self.AttackType` "NewEnumerator0"))
          (switch `/Game/Pawns/Hero/AttackType_E` _output_get
            (:`NewEnumerator0`
              (`self.PlayAnimMontage` "/Game/Pawns/Hero/Animations/hero_melee_attack_downward_Montage.hero_melee_attack_downward_Montage")
              (set `self.AttackType` "NewEnumerator5"))))))
    (:`Is Not Valid`
      (`KismetSystemLibrary.PrintString` "No Weapon Equiped"))))

(fn `UserConstructionScript`
  (`parent.UserConstructionScript`))