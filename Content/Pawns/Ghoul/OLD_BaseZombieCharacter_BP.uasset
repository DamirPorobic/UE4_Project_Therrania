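; Base zombie Character Blueprint for a Ghoul enemy, marked OLD by its file name, providing basic sight and movement-speed plumbing.
; PawnSensing stores the last seen pawn in ISeePawn, which getter and setter functions expose.
; A ChangeSpeed event scales the walk speed from SpeedVariable by a given rate.
; EnemyFound and EnemyLost are empty stubs, and BeginPlay casts the game instance.
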(event `self.ReceiveBeginPlay`
  (cast `` (`GameplayStatics.GetGameInstance`))
  (set `self.ReferenceToGameInstance` null))

(event `ChangeSpeed`
  (params (SpeedRate :type "Float (double-precision)"))
  (set `CharacterMovementComponent.MaxWalkSpeed` (* SpeedRate (`self.SpeedVariable`)) (`self.CharacterMovement`)))

(event `self.PawnSensing.OnSeePawn`
  (params (Pawn :type "Pawn Object Reference"))
  (set `self.ISeePawn` Pawn))

(fn `EnemyFound`)

(fn `EnemyLost`)

(fn `GetSeenPawn`
  (returns (SeenPawn :type "Object Object Reference"))
  (cast `` (`self.ISeePawn`)
    (:`then`
      (return null))
    (:`CastFailed`
      (return null))))

(fn `SetSeenPawn`
  (params (SeenPawn :type "Pawn Object Reference"))
  (set `self.ISeePawn` SeenPawn))

(fn `UserConstructionScript`)