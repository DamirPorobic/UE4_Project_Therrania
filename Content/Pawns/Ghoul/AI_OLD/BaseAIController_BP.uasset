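; Base AI controller for Ghoul pawns that runs a behavior tree and suspends AI logic while the game is paused.
; BeginPlay starts the tree, casts the game instance and marks AI as enabled.
; Tick polls the pause state, stopping the brain component when paused and restarting it on resume, with an AIEnabled flag guarding the restart.
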(event `self.ReceiveBeginPlay`
  (`self.RunBehaviorTree` null)
  (cast `` (`GameplayStatics.GetGameInstance`))
  (set `self.ReferenceToGameInstance` null)
  (set `self.AIEnabled` true))

(event `self.ReceiveTick`
  (params (DeltaSeconds :type "Float (single-precision)"))
  (if (`self.IsGamePaused`)
    (`BrainComponent.StopLogic` (`self.BrainComponent`) "")
    (set `self.AIEnabled` false)
    (elif (not (`self.AIEnabled`))
      (`BrainComponent.RestartLogic` (`self.BrainComponent`))
      (set `self.AIEnabled` true))))

(fn `UserConstructionScript`)