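; Character Blueprint that runs melee and magic talents, weapon drawing and spring-arm camera zoom.
; BeginUsingTalent accepts one talent at a time, sets state flags by type and draws the weapon for damage skills and spells.
; CastSpell fires the talent from the casting socket and clears that state; UseSkill only clears flags.
; Weapon state lives in Character_AnimBP, which DrawWeapon sets and GetDrawWeapon reads for the input toggle.
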(event `BeginUsingTalent`
  (params (Talent :type "/Game/Blueprints/TalentTree/BaseTalent_BP Object Reference"))
  (if (not (`self.IsExecuting`))
    (bind _output_get (set `self.ExecutingTalent` Talent))
    (switch `/Game/Blueprints/TalentTree/TalentType_E` (`/Game/Blueprints/TalentTree/BaseTalent_BP.TalentType` _output_get)
      (:`NewEnumerator0`
        (bind _asbase_melee_skill_bp (cast `/Game/Blueprints/TalentTree/BaseMeleeSkill_BP` (`self.ExecutingTalent`)))
        (switch `/Game/Blueprints/TalentTree/SkillType_E` (`/Game/Blueprints/TalentTree/BaseMeleeSkill_BP.SkillType` _asbase_melee_skill_bp)
          (:`NewEnumerator0`
            (set `self.IsUsingSword1hAttack` true)
            (set `self.IsExecuting` true)
            (`self.DrawWeapon` true))
          (:`NewEnumerator2`
            (set `self.IsUsingConditionSkill` true)
            (set `self.IsExecuting` true))))
      (:`NewEnumerator1`
        (set `self.IsCasting` true)
        (set `self.IsExecuting` true)
        (`self.DrawWeapon` true)))))

(event `CastSpell`
  (`/Game/Blueprints/TalentTree/BaseTalent_BP.UseTalent` (`self.ExecutingTalent`) (`SceneComponent.GetSocketLocation` (`self.Mesh`) "CastingSocket") (`SceneComponent.K2_GetComponentRotation` (`self.ArrowComponent`)))
  (set `self.IsCasting` false)
  (set `self.IsExecuting` false)
  (set `self.ExecutingTalent` null))

(event `UseSkill`
  (set `self.IsUsingConditionSkill` false)
  (set `self.IsUsingSword1hAttack` false)
  (set `self.IsExecuting` false)
  (set `self.ExecutingTalent` null))

(event `InputAction|DrawWeapon`
  (params (Key :type "Key Structure" :default "AnyKey"))
  (:`Pressed`
    (bind _weapondrawn (`self.GetDrawWeapon`))
    (`self.DrawWeapon` (not _weapondrawn))))

(event `InputAction|ZoomIn`
  (params (Key :type "Key Structure" :default "AnyKey"))
  (:`Pressed`
    ;[1 1 1] Check if we are still above the minZoom level, if yes, alowe zoom in.
    (if (> (`SpringArmComponent.TargetArmLength` (`self.SpringArm`)) (`self.minZoom`))
      (set `SpringArmComponent.TargetArmLength` (- (`SpringArmComponent.TargetArmLength` (`self.SpringArm`)) 100.0) (`self.SpringArm`)))))

(event `InputAction|ZoomOut`
  (params (Key :type "Key Structure" :default "AnyKey"))
  (:`Pressed`
    ;[1 1 1] Check if we are below max zoom, if yes, alowe zoom out.
    (if (< (`SpringArmComponent.TargetArmLength` (`self.SpringArm`)) (`self.maxZoom`))
      (set `SpringArmComponent.TargetArmLength` (+ (`SpringArmComponent.TargetArmLength` (`self.SpringArm`)) 100.0) (`self.SpringArm`)))))

(fn `DrawWeapon`
  (params (DrawWeapon :type Boolean))
  ;[1 1 1] Depending on the provided input, the character will pull out his weapon or put it back in.
  (bind _ascharacter_anim_bp (cast `/Game/Pawns/Character/Animations/Character_AnimBP` (`SkeletalMeshComponent.GetAnimInstance` (`self.Mesh`))))
  (`/Game/Pawns/Character/Animations/Character_AnimBP.DrawWeapon` _ascharacter_anim_bp DrawWeapon))

(fn `GetDrawWeapon`
  (returns (WeaponDrawn :type Boolean))
  (bind _ascharacter_anim_bp (cast `/Game/Pawns/Character/Animations/Character_AnimBP` (`SkeletalMeshComponent.GetAnimInstance` (`self.Mesh`)))
    (:`then`
      (return (`/Game/Pawns/Character/Animations/Character_AnimBP.InCombat` _ascharacter_anim_bp)))
    (:`CastFailed`
      (return false))))

(fn `UserConstructionScript`)